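; Player controller for the shooter that owns the game HUD, manages input for the countdown and handles leaving a multiplayer session.
; On BeginPlay the local controller clears existing widgets, shows the HUD and sets game-only input.
; It passes the HUD reference to the possessed ThirdPersonCharacter, and exposes events to start the pre-countdown, enable pawn input and unhide the HUD.
; Ending a client session flags the GameInstance, destroys the session and opens the main menu.
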(event Custom|EnableControlsWhenPreCountdownIsFinished
  ;[0.01042 0.01042 0.01042] Enable movement when pre countdown is finished
  (Input|EnableInput (Pawn|GetControlledPawn) self))

(event Custom|StartPreCountdown
  ;[0.01042 0.01042 0.01042] Enable movement when pre countdown is finished
  (Default|StartPreCountdown (Variables|Default|GetGameWidget)))

(event Custom|UnHideGameHud
  ;[0.01042 0.01042 0.01042] Un hide game hud, when closing pause menu
  (Widget|SetVisibility (Variables|Default|GetGameWidget) "Visible"))

(event Custom|EndClientSession
  ;[0.01042 0.01042 0.01042] End session
  (bind _asshooter_game_instance (Utilities|Casting|CastToShooterGameInstance (Game|GetGameInstance)))
  (Variables|/Game/Game/Blueprints/ModesAndControllers/ShooterGameInstance.ShooterGameInstance_C|SetMultiplayerShowPauseMenu _asshooter_game_instance true)
  (|DestroySession self
    (:OnSuccess
      (Game|OpenLevel(byName) "MainMenuMap"))))

(event Custom|InitHudVariablesLocal
  ;[0.01042 0.01042 0.01042] Init hud variables for standalone
  (bind _asthird_person_character (Utilities|Casting|CastToThirdPersonCharacter (Pawn|GetControlledPawn)))
  (Variables|/Game/Game/Blueprints/Characters/ThirdPersonCharacter.ThirdPersonCharacter_C|SetGameWidget _asthird_person_character (Variables|Default|GetGameWidget)))

(event EventBeginPlay
  ;[0.01042 0.01042 0.01042] Enables input when the game starts
  (if (Pawn|IsLocalController)
    (Viewport|RemoveAllWidgets)
    (CallFunction|ShowGameHud)
    (Input|SetInputModeGameOnly self)
    (Variables|Default|SetbShowMouseCursor false)))

(event EventTick
  (params (DeltaSeconds :type Float%20%28single-precision%29)))

(event EventPossess
  (params (PossessedPawn :type Pawn%20Object%20Reference))
  ;[0.01042 0.01042 0.01042] Init hud variables for standalone
  (CallFunction|InitHudVariablesLocal))

(fn ConstructionScript)

(fn ShowGameHud
  (Utilities|IsValid (Variables|Default|GetGameWidget)
    (:Is%20Valid
      _)
    (:Is%20Not%20Valid
      (bind _returnvalue (UserInterface|CreateWidget "/Game/Game/Blueprints/Widgets/GameWidget.GameWidget_C" self))
      (Variables|Default|SetGameWidget _returnvalue)))
  (UserInterface|Viewport|AddtoViewport (Variables|Default|GetGameWidget) 0))